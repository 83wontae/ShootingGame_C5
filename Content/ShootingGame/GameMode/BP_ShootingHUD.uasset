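; HUD for the shooting game that creates the on-screen widget on BeginPlay and starts in game-only input.
; It forwards ammo, magazine and message text to the widget and switches to UI-only input with a cursor for chat.
; BindPlayerState hooks player-name and HP dispatchers to refresh the player list and local health.
; Widget updates and local PlayerState binding retry on short timers until the widget or state is valid.
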(event EventBeginPlay
  (bind _returnvalue (Game|GetPlayerController 0))
  (bind _returnvalue_2 (UserInterface|CreateWidget "/Game/ShootingGame/Widget/HudWidget.HudWidget_C"))
  (bind _output_get (Variables|Default|SetHudWidget _returnvalue_2))
  (UserInterface|Viewport|AddtoViewport _output_get 0)
  (Input|SetInputModeGameOnly _returnvalue)
  (Variables|/Script/Engine.PlayerController|SetbShowMouseCursor _returnvalue false))

(fn ConstructionScript)

(fn SetAmmotoHUD
  (params (Ammo :type Integer))
  (Default|SetAmmoText (Variables|Default|GetHudWidget) Ammo))

(fn SetMagtoHUD
  (params (Mag :type Integer))
  (Default|SetMagText (Variables|Default|GetHudWidget) Mag))

(fn SetMessageText
  (params (textMessage :type Text))
  (Default|SetMessageText (Variables|Default|GetHudWidget) textMessage))

(fn SetFocusChat
  (bind _returnvalue (Game|GetPlayerController 0))
  (Input|SetInputModeUIOnly _returnvalue (Variables|Default|GetHudWidget) "DoNotLock")
  (Variables|/Script/Engine.PlayerController|SetbShowMouseCursor _returnvalue true))

(fn UpdatePlayers
  (params (PlayerName :type String))
  (CallFunction|ExUpdatePlayers))

(fn BindPlayerState
  (params (PlayerState :type BP%20Shooting%20Player%20State%20Object%20Reference))
  (Utilities|FlowControl|Sequence
    (:then_0
      (EventDispatchers|BindEventtoEventDispatcherPlayerName PlayerState (EventDispatchers|CreateEvent :!event UpdatePlayers))
      (CallFunction|UpdatePlayers))
    (:then_1
      (CallFunction|ExBindPlayerState))))

(fn ExUpdatePlayers
  (bind _hudwidget (Variables|Default|GetHudWidget))
  (Utilities|IsValid _hudwidget
    (:Is%20Valid
      (Default|UpdatePlayers _hudwidget))
    (:Is%20Not%20Valid
      (Utilities|Time|SetTimerbyFunctionName 0 "ExUpdatePlayers" 0.1))))

(fn UpdateMyHP
  (params (CurHP :type Float%20%28single-precision%29) (MaxHP :type Float%20%28single-precision%29))
  (CallFunction|ExUpdateMyHP))

(fn ExUpdateMyHP
  (bind _hudwidget (Variables|Default|GetHudWidget))
  (Utilities|IsValid _hudwidget
    (:Is%20Valid
      (bind _asbp_shooting_player_state (Utilities|Casting|CastToBP_ShootingPlayerState (Variables|/Script/Engine.Controller|GetPlayerState (Game|GetPlayerController 0))))
      (Default|SetMyHP _hudwidget (Variables|/Game/ShootingGame/GameMode/BP_ShootingPlayerState.BP_ShootingPlayerState_C|GetCurHp _asbp_shooting_player_state) (Variables|/Game/ShootingGame/GameMode/BP_ShootingPlayerState.BP_ShootingPlayerState_C|GetMaxHp _asbp_shooting_player_state)))
    (:Is%20Not%20Valid
      (Utilities|Time|SetTimerbyFunctionName 0 "ExUpdateMyHP" 0.1))))

(fn ExBindPlayerState
  (bind _returnvalue (Game|GetPlayerController 0))
  (bind _playerstate (Variables|/Script/Engine.Controller|GetPlayerState _returnvalue))
  (Utilities|IsValid _playerstate
    (:Is%20Valid
      (bind _asbp_shooting_player_state (Utilities|Casting|CastToBP_ShootingPlayerState _playerstate))
      (EventDispatchers|BindEventtoEventDispatcherUpdateHP _asbp_shooting_player_state (EventDispatchers|CreateEvent :!event UpdateMyHP))
      (CallFunction|UpdateMyHP (Variables|/Game/ShootingGame/GameMode/BP_ShootingPlayerState.BP_ShootingPlayerState_C|GetCurHp _asbp_shooting_player_state) (Variables|/Game/ShootingGame/GameMode/BP_ShootingPlayerState.BP_ShootingPlayerState_C|GetMaxHp _asbp_shooting_player_state))
      (Development|PrintString "Update HP Bind!!!" true true "(R=0.000000,G=0.500000,B=0.000000,A=1.000000)" 6e+01))
    (:Is%20Not%20Valid
      (Utilities|Time|SetTimerbyFunctionName 0 "ExBindPlayerState" 0.1))))
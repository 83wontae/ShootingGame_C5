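; Player state for the shooting game that holds each player's health and display name, with health set to max on BeginPlay.
; Setters and AddDamage change the values, and RepNotify handlers push them to the ShootingCharacter's health and name displays.
; The name notify also refreshes the HUD's player list, while the health notify prints a debug message.
; If the pawn cast fails, short timers retry the display update until it succeeds.
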(event EventBeginPlay
  (CallFunction|SetHp (Variables|Default|GetMaxHp)))

(fn ConstructionScript)

(fn OnRepCurHp
  (Development|PrintString (Utilities|String|Append (Utilities|GetDisplayName (Variables|Default|GetPawnPrivate)) " CurHp - " (Utilities|String|ToString(Float) (Variables|Default|GetCurHp))) true true "(R=0.000000,G=0.660000,B=1.000000,A=1.000000)" 6e+01)
  (bind _asshooting_character (Utilities|Casting|CastToShootingCharacter (Variables|Default|GetPawnPrivate))
    (:then
      (Default|SetProgressHp _asshooting_character))
    (:CastFailed
      (CallFunction|UpdatePlayer))))

(fn SetHp
  (params (CurHp :type Float%20%28single-precision%29))
  (bind _output_get (Variables|Default|SetCurHp CurHp))
  (return _output_get (Variables|Default|GetMaxHp)))

(fn AddDamage
  (params (Damage :type Float%20%28single-precision%29))
  (Variables|Default|SetCurHp (- (Variables|Default|GetCurHp) Damage)))

(fn UpdatePlayer
  (bind _asshooting_character (Utilities|Casting|CastToShootingCharacter (Variables|Default|GetPawnPrivate))
    (:then
      (Default|SetProgressHp _asshooting_character))
    (:CastFailed
      (Utilities|Time|SetTimerbyFunctionName 0 "UpdatePlayer" 0.1))))

(fn OnRepStrPlayerName
  (bind _asbp_shooting_hud (Utilities|Casting|CastToBP_ShootingHUD (HUD|GetHUD (Game|GetPlayerController 0))))
  (Default|UpdatePlayers _asbp_shooting_hud)
  (CallFunction|UpdatePlayerName))

(fn SetNewPlayerName
  (params (StrPlayerName :type String))
  (Variables|Default|SetStrPlayerName StrPlayerName))

(fn UpdatePlayerName
  (bind _asshooting_character (Utilities|Casting|CastToShootingCharacter (Variables|Default|GetPawnPrivate))
    (:then
      (Default|SetPlayerName _asshooting_character))
    (:CastFailed
      (Utilities|Time|SetTimerbyFunctionName 0 "UpdatePlayerName" 0.1))))
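; Lobby game mode that handles players joining and leaving the lobby.
; HandleStartingNewPlayer calls the parent implementation, then casts the player to BP_LobbyPlayerController and calls ResStartNewPlayer on it.
; PostLogin, HandleStartingNewPlayer and OnLogout each print the controller's display name on screen as a long-lived debug trace of the connection flow.
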(event EventBeginPlay)

(event EventTick
  (params (DeltaSeconds :type Float%20%28single-precision%29)))

(event EventPostLogin
  (params (NewPlayer :type Player%20Controller%20Object%20Reference))
  (Development|PrintString (Utilities|String|Append "OnPostLogin - " (Utilities|GetDisplayName NewPlayer)) true true "(R=0.000000,G=0.660000,B=1.000000,A=1.000000)" 6e+01))

(event EventHandleStartingNewPlayer
  (params (NewPlayer :type Player%20Controller%20Object%20Reference))
  ;[1 1 1] 캐릭터 안나오시는 분은 요거 넣어주세요
  (|CallParentFunction NewPlayer)
  (Development|PrintString (Utilities|String|Append "Handle Starting New Player - " (Utilities|GetDisplayName NewPlayer)) true true "(R=0.000000,G=0.660000,B=1.000000,A=1.000000)" 6e+01)
  (bind _asbp_lobby_player_controller (Utilities|Casting|CastToBP_LobbyPlayerController NewPlayer))
  (Default|ResStartNewPlayer _asbp_lobby_player_controller))

(event EventOnLogout
  (params (ExitingController :type Controller%20Object%20Reference))
  (Development|PrintString (Utilities|String|Append "OnLogout - " (Utilities|GetDisplayName ExitingController)) true true "(R=0.000000,G=0.660000,B=1.000000,A=1.000000)" 6e+01))

(fn ConstructionScript)
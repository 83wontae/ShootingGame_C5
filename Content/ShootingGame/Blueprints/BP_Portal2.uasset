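; BP_Portal2 is a portal actor that reveals its Sphere once every BP_HitActor in the level is fractured.
; On BeginPlay it hides the Sphere, disables its collision and binds to each hit actor's Hit dispatcher.
; CheckAllHitActors scans all hit actors' IsFracture flags and, if all are set, restores visibility and query-and-physics collision.
; The portal has no overlap behavior of its own.
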(event EventBeginPlay
  (bind _sphere (Variables|Default|GetSphere))
  (Rendering|SetVisibility _sphere false false)
  (Collision|SetCollisionEnabled _sphere "NoCollision")
  (CallFunction|BindHitActors))

(event Collision|EventActorBeginOverlap
  (params (OtherActor :type Actor%20Object%20Reference)))

(event EventTick
  (params (DeltaSeconds :type Float%20%28single-precision%29)))

(fn ConstructionScript)

(fn BindHitActors
  (bind _outactors (Actor|GetAllActorsOfClass "/Game/ShootingGame/Blueprints/BP_HitActor.BP_HitActor_C"))
  (for _array_element _outactors
    (EventDispatchers|BindEventtoEventDispatcherHit _array_element (EventDispatchers|CreateEvent :!event CheckAllHitActors))))

(fn CheckAllHitActors
  (bind _sphere (Variables|Default|GetSphere))
  (bind _isallfacture (CallFunction|IsAllHitActors))
  (if _isallfacture
    (Rendering|SetVisibility _sphere true false)
    (Collision|SetCollisionEnabled _sphere "QueryAndPhysics")))

(fn IsAllHitActors
  (bind _outactors (Actor|GetAllActorsOfClass "/Game/ShootingGame/Blueprints/BP_HitActor.BP_HitActor_C"))
  (for _array_element _outactors
    (if (not (Variables|/Game/ShootingGame/Blueprints/BP_HitActor.BP_HitActor_C|GetIsFracture _array_element))
      (return false)))
  (return true))
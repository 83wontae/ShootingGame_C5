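; BP_MoveRect is a shooting-game actor whose Cube travels around a rectangular loop in the local XZ plane while its switch is overlapped.
; BeginPlay binds to the Switch's overlap dispatcher, and EventSwitchOverlap starts or clears a looping UpdateMove timer on begin or end.
; UpdateMove steps the cube according to MoveType, cycling Right, Up, Left and Down as its relative position passes Dist or zero.
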(event EventBeginPlay
  (EventDispatchers|BindEventtoEventDispatcherOverlap (Variables|Default|GetSwitch) (EventDispatchers|CreateEvent :!event EventSwitchOverlap)))

(fn ConstructionScript)

(fn UpdateMove
  (switch Utilities|FlowControl|Switch|SwitchonEN_MoveType (Variables|Default|GetMoveType)
    (:NewEnumerator0
      (CallFunction|MoveRight))
    (:NewEnumerator1
      (CallFunction|MoveUp))
    (:NewEnumerator2
      (CallFunction|MoveLeft))
    (:NewEnumerator3
      (CallFunction|MoveDown))))

(fn MoveRight
  ;[1 1 1] 오른쪽으로 이동
  (Transformation|AddRelativeLocation (Variables|Default|GetCube) "5.000000, 0, 0" false false)
  (if (> (.x (Variables|/Script/Engine.SceneComponent|GetRelativeLocation (Variables|Default|GetCube))) (Variables|Default|GetDist))
    (Variables|Default|SetMoveType "NewEnumerator1")))

(fn MoveUp
  ;[1 1 1] 위로 이동
  (Transformation|AddRelativeLocation (Variables|Default|GetCube) "0.000000, 0,5.000000" false false)
  (if (> (.z (Variables|/Script/Engine.SceneComponent|GetRelativeLocation (Variables|Default|GetCube))) (Variables|Default|GetDist))
    (Variables|Default|SetMoveType "NewEnumerator2")))

(fn MoveLeft
  ;[1 1 1] 왼쪽으로 이동
  (Transformation|AddRelativeLocation (Variables|Default|GetCube) "-5.000000, 0, 0" false false)
  (if (< (.x (Variables|/Script/Engine.SceneComponent|GetRelativeLocation (Variables|Default|GetCube))) 0.0)
    (Variables|Default|SetMoveType "NewEnumerator3")))

(fn MoveDown
  ;[1 1 1] 아래로 이동
  (Transformation|AddRelativeLocation (Variables|Default|GetCube) "0.000000, 0,-5.000000" false false)
  (if (< (.z (Variables|/Script/Engine.SceneComponent|GetRelativeLocation (Variables|Default|GetCube))) 0.0)
    (Variables|Default|SetMoveType "NewEnumerator0")))

(fn DoPlay
  (Utilities|Time|SetTimerbyFunctionName 0 "UpdateMove" 0.01 true))

(fn DoStop
  (Utilities|Time|ClearTimerbyFunctionName 0 "UpdateMove"))

(fn EventSwitchOverlap
  (params (IsBegin :type Boolean))
  (if IsBegin
    (CallFunction|DoPlay)
    (else
      (CallFunction|DoStop))))
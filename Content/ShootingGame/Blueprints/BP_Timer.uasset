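; BP_Timer is a play timer in the shooting game that counts elapsed time while a linked Switch is overlapped.
; On BeginPlay it binds to the Switch's overlap event dispatcher, with EventSwitchOverlap setting IsPlay from the overlap begin state.
; Tick accumulates delta seconds while playing and prints the Korean minutes-and-seconds string only when it differs from the last one.
; The total is never reset, so timing resumes where it paused.
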(event EventBeginPlay
  (EventDispatchers|BindEventtoEventDispatcherOverlap (Variables|Default|GetSwitch) (EventDispatchers|CreateEvent :!event EventSwitchOverlap)))

(event EventTick
  (params (DeltaSeconds :type Float%20%28single-precision%29))
  (if (Variables|Default|GetIsPlay)
    (bind _output_get (Variables|Default|SetTotalTime (+ (* DeltaSeconds 1.0) (Variables|Default|GetTotalTime))))
    (if (not (Utilities|Enum|Equal(Enum) (Variables|Default|GetBeforeStr) (Utilities|String|Append (Utilities|String|ToString(Integer) (Math|Float|Floor (/ _output_get 6e+01))) "분" (Utilities|String|ToString(Integer) (Math|Float|Floor (Math|Float|%(Float) _output_get 6e+01))) "초")))
      (Development|PrintString (Utilities|String|Append (Utilities|String|ToString(Integer) (Math|Float|Floor (/ _output_get 6e+01))) "분" (Utilities|String|ToString(Integer) (Math|Float|Floor (Math|Float|%(Float) _output_get 6e+01))) "초"))
      (Variables|Default|SetBeforeStr (Utilities|String|Append (Utilities|String|ToString(Integer) (Math|Float|Floor (/ _output_get 6e+01))) "분" (Utilities|String|ToString(Integer) (Math|Float|Floor (Math|Float|%(Float) _output_get 6e+01))) "초")))))

(fn ConstructionScript)

(fn EventSwitchOverlap
  (params (IsBegin :type Boolean))
  (Variables|Default|SetIsPlay IsBegin))
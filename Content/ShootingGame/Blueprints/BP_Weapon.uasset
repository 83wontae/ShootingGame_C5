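; BP_Weapon is a rifle that a character can attach to its hand socket "weapon" or drop as a physics object.
; A trigger press plays the owner's fire montage if ammo remains, while the shot itself runs separately in NotifyFire.
; NotifyFire spends ammo, updates the HUD, plays muzzle effects and line-traces from the camera, applying destructible damage to any BP_HitActor's rock.
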(event EventPressedTrigger
  (CallFunction|PlayFire))

(fn ConstructionScript)

(fn UseAmmo
  (Math|Integer|DecrementInt (Variables|Default|GetAmmo)
    (:%20%20
      (bind _asbp_shooting_hud (Utilities|Casting|CastToBP_ShootingHUD (HUD|GetHUD (Game|GetPlayerController 0))))
      (Default|SetAmmotoHUD _asbp_shooting_hud (Variables|Default|GetAmmo)))))

(fn IsCanFire
  (return (> (Variables|Default|GetAmmo) 0)))

(fn PlayFire
  (if (CallFunction|IsCanFire)
    (Animation|PlayAnimMontage (Variables|Default|GetOwnCharacter) "/Game/RifleAnimsetPro/Animations/InPlace/Rifle_ShootOnce_Montage_InPlace.Rifle_ShootOnce_Montage_InPlace" 1.0 "None")))

(fn AttachtoChar
  (params (Character :type Character%20Object%20Reference))
  (bind _staticmesh (Variables|Default|GetStaticMesh))
  (Physics|SetSimulatePhysics _staticmesh false)
  (Collision|SetCollisionEnabled _staticmesh "NoCollision")
  (bind _returnvalue (Transformation|AttachComponentToComponent _staticmesh (Variables|/Script/Engine.Character|GetMesh Character) "weapon" "SnapToTarget" "SnapToTarget" "KeepWorld" true))
  (if _returnvalue
    (Variables|Default|SetOwnCharacter Character)
    (return _returnvalue)
    (else
      (return _returnvalue))))

(fn DetachtoChar
  (params (Character :type Character%20Object%20Reference))
  (bind _staticmesh (Variables|Default|GetStaticMesh))
  (Transformation|DetachFromComponent (Variables|Default|GetStaticMesh) "KeepWorld" "KeepWorld" "KeepWorld" true)
  (Collision|SetCollisionEnabled _staticmesh "QueryAndPhysics")
  (Physics|SetSimulatePhysics _staticmesh true)
  (Variables|Default|SetOwnCharacter 0)
  (return true))

(fn NotifyFire
  (bind _returnvalue (Game|GetPlayerCameraManager 0))
  (bind _staticmesh (Variables|Default|GetStaticMesh))
  (bind _returnvalue_2 (Transformation|GetActorLocation _returnvalue))
  (CallFunction|UseAmmo)
  (Effects|SpawnEmitteratLocation "/Game/StarterContent/Particles/P_Explosion.P_Explosion" (Transformation|GetSocketLocation _staticmesh "Muzzle") (Transformation|GetSocketRotation _staticmesh "Muzzle") "0.100000,0.100000,0.100000")
  (Audio|SpawnSoundatLocation "/Game/StarterContent/Audio/Explosion_Cue.Explosion_Cue" (Transformation|GetSocketLocation (Variables|Default|GetStaticMesh) "Muzzle") "0, 0, 0" 1.0 1.0 0.0 0 0)
  (bind (_outhit _returnvalue_3) (Collision|LineTraceForObjects (+ _returnvalue_2 (* (Transformation|GetActorForwardVector _returnvalue) 3e+02)) (+ _returnvalue_2 (* (Transformation|GetActorForwardVector _returnvalue) 1e+04)) (Utilities|Array|MakeArray "ObjectTypeQuery1" "ObjectTypeQuery2" "ObjectTypeQuery3" "ObjectTypeQuery4" "ObjectTypeQuery6") false 0 "ForDuration"))
  (if _returnvalue_3
    (bind _asbp_hit_actor (Utilities|Casting|CastToBP_HitActor (.HitActor (Collision|BreakHitResult _outhit))))
    (Class|DestructibleComponent|ApplyDamage (Variables|/Game/ShootingGame/Blueprints/BP_HitActor.BP_HitActor_C|GetRock _asbp_hit_actor) 1e+03 (.ImpactPoint (Collision|BreakHitResult _outhit)) (.ImpactNormal (Collision|BreakHitResult _outhit)) 5e+04)
    (return true)))
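; BP_MoveLeftRight is a shooting-game actor that slides a Cube back and forth along its relative X axis within Dist.
; A Switch reference's overlap dispatcher is bound on BeginPlay, and EventSwitchOverlap starts or stops a looping timer on begin or end.
; The timer calls UpdateMove, stepping the Cube and flipping IsRight at each limit.
; A separate L-key timeline path also sets the Cube's position and reverses on finish.
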(event EventBeginPlay
  (EventDispatchers|BindEventtoEventDispatcherOverlap (Variables|Default|GetSwitch) (EventDispatchers|CreateEvent :!event EventSwitchOverlap)))

(event Input|KeyboardEvents|L
  (params (Key :type Key%20Structure :default "None"))
  ;[1 1 1] 타임라인
  (:Pressed
    (bind _value (Timeline|타임라인_0 SetNewTime)
      (:Update
        (Transformation|SetRelativeLocation (Variables|Default|GetCube) (Math|Vector|MakeVector (* _value (Variables|Default|GetDist)) 0.0 0.0) false false))
      (:Finished
        (Variables|Default|SetIsRight (not (Variables|Default|GetIsRight)))
        (if (Variables|Default|GetIsRight)
          (Timeline|타임라인_0 Play)
          (else
            (Timeline|타임라인_0 Reverse)))))))

(fn ConstructionScript)

(fn UpdateMove
  (if (Variables|Default|GetIsRight)
    (Transformation|AddRelativeLocation (Variables|Default|GetCube) "5.000000, 0, 0" false false)
    (if (> (.x (Variables|/Script/Engine.SceneComponent|GetRelativeLocation (Variables|Default|GetCube))) (Variables|Default|GetDist))
      (Variables|Default|SetIsRight false))
    (else
      (Transformation|AddRelativeLocation (Variables|Default|GetCube) "-5.000000, 0, 0" false false)
      (if (< (.x (Variables|/Script/Engine.SceneComponent|GetRelativeLocation (Variables|Default|GetCube))) 0.0)
        (Variables|Default|SetIsRight true)))))

(fn DelayPrintString
  (Development|PrintString "Delay")
  (Utilities|Time|ClearTimerbyFunctionName 0 "UpdateMove"))

(fn DoPlay
  (Utilities|Time|SetTimerbyFunctionName 0 "UpdateMove" 0.01 true))

(fn DoStop
  (Utilities|Time|ClearTimerbyFunctionName 0 "UpdateMove"))

(fn EventSwitchOverlap
  (params (IsBegin :type Boolean))
  (if IsBegin
    (CallFunction|DoPlay)
    (else
      (CallFunction|DoStop))))
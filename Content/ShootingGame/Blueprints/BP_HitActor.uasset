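; BP_HitActor is a fracturable rock actor that reports when it takes damage or breaks in the shooting game.
; AnyDamage only prints the damage amount, type, instigator and causer to the screen for debugging.
; When the Rock component fractures, it prints a message, sets IsFracture and fires the Hit event dispatcher; BeginPlay initializes that flag to false.
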(event OnComponentFracture(Rock)
  (params (HitPoint :type Vector%20%28by%20ref%29 :default "0, 0, 0") (HitDirection :type Vector%20%28by%20ref%29 :default "0, 0, 0"))
  (Development|PrintString "Fracture!!!")
  (Variables|Default|SetIsFracture true)
  (Default|CallEventDispatcherHit))

(event EventBeginPlay
  (Variables|Default|SetIsFracture false))

(event Game|Damage|EventAnyDamage
  (params (Damage :type Float%20%28single-precision%29) (DamageType :type Damage%20Type%20Object%20Reference) (InstigatedBy :type Controller%20Object%20Reference) (DamageCauser :type Actor%20Object%20Reference))
  (Development|PrintString (Utilities|String|Append "AnyDamage Damage :" (Utilities|String|ToString(Float) Damage) ", DmageType :" (Utilities|GetDisplayName DamageType) ", InstigatedBy :" (Utilities|GetDisplayName InstigatedBy) ", DamageCauser :" (Utilities|GetDisplayName DamageCauser)) true true "(R=0.000000,G=0.660000,B=1.000000,A=1.000000)" 6e+01))

(fn ConstructionScript)